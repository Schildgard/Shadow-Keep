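; Behavior tree task that times an enemy's strafe phase; the file itself contains no movement logic.
; On execute it casts the controlled pawn to Enemy and stores it, only logging if the cast fails.
; Tick counts down StrafeTime, resets it on expiry, then calls ResetAttackState2 on a valid Enemy and finishes successfully.
; An invalid Enemy only logs, leaving the task unfinished.
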(event `self.ReceiveExecuteAI`
  (params (OwnerController :type "AIController Object Reference") (ControlledPawn :type "Pawn Object Reference"))
  (bind _asenemy (cast `Enemy` ControlledPawn)
    (:`then`
      (set `self.Enemy` _asenemy))
    (:`CastFailed`
      (`KismetSystemLibrary.LogString` "Cast Fail (Behaviour Tree)"))))

(event `self.ReceiveTick`
  (params (OwnerActor :type "Actor Object Reference") (DeltaSeconds :type "Float (single-precision)"))
  (bind _enemy (`self.Enemy`))
  (set `self.StrafeTime` (- (`self.StrafeTime`) DeltaSeconds))
  (if (<= (`self.StrafeTime`) 0.0)
    (`KismetSystemLibrary.LogString` "StrafeTimer is Over")
    (set `self.StrafeTime` (`self.StrafeTimeMax`))
    (`/Engine/EditorBlueprintResources/StandardMacros.IsValid` _enemy
      (:`Is Valid`
        (`NPCBase.ResetAttackState2` _enemy)
        (`self.FinishExecute` true))
      (:`Is Not Valid`
        (`KismetSystemLibrary.LogString` "Super fail (Strafe Task)")))))